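; AI controller for enemies that runs the BT_Enemy behavior tree and feeds its blackboard.
; On BeginPlay it copies the controlled RP_Enemy's path settings (looping, direction index, wait time at path points) into blackboard keys.
; Perception updates set bCanSeePlayer from the stimulus's sensed state, only for RP_Character actors of the player type.
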(event `self.ReceiveBeginPlay`
  (`self.RunBehaviorTree` "/Game/BluePrints/AI/BT_Enemy.BT_Enemy")
  (bind _asrp_enemy (cast `RP_Enemy` (`self.K2_GetPawn`)))
  (`BlackboardComponent.SetValueAsBool` (`AIBlueprintHelperLibrary.GetBlackboard` null) "bLoopPath" (`RP_Enemy.bLoopPath` _asrp_enemy))
  (`BlackboardComponent.SetValueAsInt` (`AIBlueprintHelperLibrary.GetBlackboard` null) "DirectionIndex" (`RP_Enemy.DirectionIndex` _asrp_enemy))
  (`BlackboardComponent.SetValueAsFloat` (`AIBlueprintHelperLibrary.GetBlackboard` null) "WaitingOnPathPoint" (`RP_Enemy.WaitingTimeOnPathPoint` _asrp_enemy)))

(event `self.AIPerception.OnTargetPerceptionUpdated`
  (params (Actor :type "Actor Object Reference") (Stimulus :type "AIStimulus Structure"))
  (bind _asrp_character (cast `RP_Character` Actor))
  (bind _returnvalue (`RP_Character.GetCharacterType` _asrp_character))
  (if (`|EnumEquality` _returnvalue "CharacterType_Player")
    (`BlackboardComponent.SetValueAsBool` (`AIBlueprintHelperLibrary.GetBlackboard` null) "bCanSeePlayer" (`.bSuccessfullySensed` (break `AIStimulus` Stimulus)))))

(fn `UserConstructionScript`)