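; Player character Blueprint with first- or third-person view, two ultimate abilities and a pause menu.
; BeginPlay creates the HUD and caches the default post-process settings, which ultimate start/stop events swap with per-ultimate looks.
; The pause input reuses one menu widget while toggling pause, cursor and input mode; the construction script sets camera auto-activation from UseFirstPersonView.
; XP and duration events are empty here, with disconnected debug prints and an H-key XP cheat.
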(event `self.BP_UpdateUltimateDuration`
  (params (Value :type "Float (single-precision)")))

(event `self.BP_UpdateUltimateDuration2`
  (params (Value :type "Float (single-precision)")))

(event `self.BP_StartUltimate2`
  (set `PostProcessComponent.Settings` (`self.Ultimate2PostProcess`) (`self.PostProcess`)))

(event `self.BP_StopUltimate2`
  (set `PostProcessComponent.Settings` (`self.NormalPostProcess`) (`self.PostProcess`)))

(event `self.BP_StartUltimate`
  (set `PostProcessComponent.Settings` (`self.UltimatePostProcess`) (`self.PostProcess`)))

(event `self.BP_StopUltimate`
  (set `PostProcessComponent.Settings` (`self.NormalPostProcess`) (`self.PostProcess`)))

(event `self.ReceiveBeginPlay`
  (`|ExecutionSequence`
    (:`then_0`
      (bind _returnvalue (`|CreateWidget` "/Game/BluePrints/UI/HUD/W_MainHUD.W_MainHUD_C"))
      (`UserWidget.AddToViewport` _returnvalue 0))
    (:`then_1`
      (set `self.NormalPostProcess` (`PostProcessComponent.Settings` (`self.PostProcess`))))))

(event `self.BP_GainUltimateXP`
  (params (XPGained :type "Float (single-precision)")))

(event `InputAction|PauseGame` :paused true
  (params (Key :type "Key Structure"))
  (bind _returnvalue (`GameplayStatics.GetPlayerController` 0))
  (bind _pause_menu_ref (`self.Pause Menu REF`))
  (:`Pressed`
    (`/Engine/EditorBlueprintResources/StandardMacros.IsValid` (`self.Pause Menu REF`)
      (:`Is Valid`
        _)
      (:`Is Not Valid`
        (bind _returnvalue_2 (`|CreateWidget` "/Game/BluePrints/UI/Pause/W_PauseMenu.W_PauseMenu_C"))
        (set `self.Pause Menu REF` _returnvalue_2)))
    (if (`GameplayStatics.IsGamePaused`)
      (`Widget.RemoveFromParent` _pause_menu_ref)
      (`GameplayStatics.SetGamePaused` false)
      (set `PlayerController.bShowMouseCursor` false _returnvalue)
      (`WidgetBlueprintLibrary.SetInputMode_GameOnly` _returnvalue)
      (else
        (`UserWidget.AddToViewport` _pause_menu_ref 0)
        (`GameplayStatics.SetGamePaused` true)
        (set `PlayerController.bShowMouseCursor` true _returnvalue)
        (`WidgetBlueprintLibrary.SetInputMode_GameAndUIEx` _returnvalue _pause_menu_ref "LockInFullscreen" false)))))

(event `Key|H`
  (params (Key :type "Key Structure"))
  (:`Pressed`
    (`self.GainUltimateXP` 10000.0)))

(fn `UserConstructionScript`
  (`ActorComponent.SetAutoActivate` (`self.FPSCameraComponent`) (`self.bUseFirstPersonView`))
  (`ActorComponent.SetAutoActivate` (`self.TPSCameraComponent`) (not (`self.bUseFirstPersonView`)))
  (`ActorComponent.SetAutoActivate` (`self.SpringArmComponent`) (not (`self.bUseFirstPersonView`))))